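; Zombie AI enemy that runs a behavior tree through its AI controller and deals area damage.
; Any overlap with its DamageCollision sphere triggers radial damage sized to that sphere's radius, ignoring all BP_AdvancedAI instances.
; When damaged, it has a small random chance to have the damage-causing PlayerPawn play a zombie growl at the zombie's location.
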(event OnComponentBeginOverlap(DamageCollision)
  (params (OverlappedComponent :type Primitive%20Component%20Object%20Reference) (OtherActor :type Actor%20Object%20Reference) (OtherComp :type Primitive%20Component%20Object%20Reference) (OtherBodyIndex :type Integer) (bFromSweep :type Boolean) (SweepResult :type Hit%20Result%20Structure%20%28by%20ref%29))
  ;[1 1 1] Tell server we want to deal player damage
  (CallFunction|ZombieRadialDamage))

(event Custom|ZombieRadialDamage
  (bind _self self)
  ;[1 1 1] Tell server we want to deal player damage
  (bind _outactors (Actor|GetAllActorsOfClass "BP_AdvancedAI_C"))
  (Game|Damage|ApplyRadialDamage 25.0 (Transformation|GetActorLocation _self) (Components|Sphere|GetScaledSphereRadius (Variables|Default|GetDamageCollision)) 0 _outactors _self 0 true "ECC_WorldDynamic"))

(event EventBeginPlay
  ;[1 1 1] Assign AI Tree on spawn
  (AI|RunBehaviorTree (AI|GetAIController self) "/Game/AdvancedAI/BT_AdvancedAI.BT_AdvancedAI"))

(event Game|Damage|EventAnyDamage
  (params (Damage :type Float%20%28single-precision%29) (DamageType :type Damage%20Type%20Object%20Reference) (InstigatedBy :type Controller%20Object%20Reference) (DamageCauser :type Actor%20Object%20Reference))
  ;[1 1 1] Play Sound On Damage
  (if (>= (Math|Random|RandomIntegerinRange 0 100) 85)
    (bind _asplayer_pawn (Utilities|Casting|CastToPlayerPawn DamageCauser))
    (Default|PlaySound _asplayer_pawn (Transformation|GetActorLocation) "/Game/Sounds/Zombies/ZombieGrowl.ZombieGrowl")))

(fn ConstructionScript)