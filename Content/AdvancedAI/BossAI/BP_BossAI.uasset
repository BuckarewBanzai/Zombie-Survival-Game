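; Boss zombie AI that runs the BT_AdvancedAI behavior tree on BeginPlay.
; During a boss fight it doubles in scale and sets its health from the wave count and number of player pawns.
; Any overlap with its damage sphere triggers full radial damage around it, ignoring BP_AdvancedAI actors.
; When damaged, it occasionally has the attacking player pawn play a growl at its location.
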(event OnComponentBeginOverlap(DamageCollision)
  (params (OverlappedComponent :type Primitive%20Component%20Object%20Reference) (OtherActor :type Actor%20Object%20Reference) (OtherComp :type Primitive%20Component%20Object%20Reference) (OtherBodyIndex :type Integer) (bFromSweep :type Boolean) (SweepResult :type Hit%20Result%20Structure%20%28by%20ref%29))
  ;[1 1 1] Tell server we want to deal player damage
  (CallFunction|ZombieRadialDamage))

(event Custom|ZombieRadialDamage
  (bind _self self)
  ;[1 1 1] Tell server we want to deal player damage
  (bind _outactors (Actor|GetAllActorsOfClass "/Game/AdvancedAI/BP_AdvancedAI.BP_AdvancedAI_C"))
  (Game|Damage|ApplyRadialDamage 1e+02 (Transformation|GetActorLocation _self) (Components|Sphere|GetScaledSphereRadius (Variables|Default|GetDamageCollision)) 0 _outactors _self 0 true "ECC_WorldDynamic"))

(event Custom|SetBossHealth
  (params (BossHealthInput :type Float%20%28single-precision%29))
  (bind _healthcomp (Variables|Default|GetHealthComp))
  (bind _output_get (Variables|/Script/CoopGame.SHealthComponent|SetDefaultHealth _healthcomp BossHealthInput))
  (Development|PrintString (Utilities|String|ToString(Float) _output_get))
  (Variables|/Script/CoopGame.SHealthComponent|SetHealth _healthcomp _output_get))

(event Custom|SetBossHealthServer
  (params (BossHealthInput :type Float%20%28single-precision%29))
  (CallFunction|SetBossHealth BossHealthInput))

(event EventBeginPlay
  (AI|RunBehaviorTree (AI|GetAIController self) "/Game/AdvancedAI/BT_AdvancedAI.BT_AdvancedAI")
  (bind _asbp_test_game_mode (Utilities|Casting|CastToBP_TestGameMode (Game|GetGameMode)))
  (if (Variables|/Game/Blueprints/GameModes/BP_TestGameMode.BP_TestGameMode_C|GetIsBossFight _asbp_test_game_mode)
    (Transformation|SetActorScale3D "2.000000,2.000000,2.000000")
    (bind _outactors (Actor|GetAllActorsOfClass "/Game/Blueprints/Player/PlayerPawn.PlayerPawn_C"))
    (bind _asbp_test_game_mode_2 (Utilities|Casting|CastToBP_TestGameMode (Game|GetGameMode)))
    (CallFunction|SetBossHealthServer (Math|Conversions|ToFloat(Integer) (+ (* (Variables|/Script/CoopGame.SGameMode|GetWaveCount _asbp_test_game_mode_2) 2500) (* (Utilities|Array|Length _outactors) 3000))))))

(event Game|Damage|EventAnyDamage
  (params (Damage :type Float%20%28single-precision%29) (DamageType :type Damage%20Type%20Object%20Reference) (InstigatedBy :type Controller%20Object%20Reference) (DamageCauser :type Actor%20Object%20Reference))
  ;[1 1 1] On Damage
  (if (>= (Math|Random|RandomIntegerinRange 0 100) 85)
    (bind _asplayer_pawn (Utilities|Casting|CastToPlayerPawn DamageCauser))
    (Default|PlaySound _asplayer_pawn (Transformation|GetActorLocation) "/Game/Sounds/Zombies/ZombieGrowl.ZombieGrowl")))

(fn ConstructionScript)