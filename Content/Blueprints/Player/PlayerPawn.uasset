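; Player character Blueprint that adds a local crosshair, score text, overhead name/health tag and wave-start drums.
; BeginPlay loads color and name from the PlayerMenuData save, and damage updates the health bar value.
; RepNotify variables drive the dynamic body material and rebuild the nametag widget, while death copies the name to SPlayerState.
; When dead, F cycles the view target through living players, routing remote calls through ServerSetViewTarget and using player index 0.
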(event Custom|PlayWaveStart
  ;[1 1 1] Audio Handling
  (Audio|PlaySoundatLocation "/Game/Sounds/Announcer/Tribal_Drums_Sound_Effect.Tribal_Drums_Sound_Effect" (Transformation|GetActorLocation) "0, 0, 0" 1.0 1.0 0.0 0 0 0))

(event Custom|PlaySound
  (params (LocationInput :type Vector) (SoundInput :type Sound%20Base%20Object%20Reference))
  ;[1 1 1] Audio Handling
  (Audio|PlaySoundatLocation SoundInput LocationInput "0, 0, 0" 1.0 1.0 0.0 "/Game/TrackerBot/TrackerBotAttenuation.TrackerBotAttenuation" 0 0))

(event Custom|SpawnSpectatePawn
  (bind _returnvalue (Game|GetPlayerController 0))
  ;[1 1 1] Spawn Spectate Pawn
  (bind _returnvalue_2 (Game|SpawnActorfromClass "/Script/Engine.SpectatorPawn" (Transformation|GetActorTransform (Game|Player|GetPlayerPawn 0)) "Undefined" 0 0))
  (Pawn|Possess _returnvalue _returnvalue_2)
  (Input|SetInputModeGameOnly _returnvalue))

(event EventBeginPlay
  ;[1 1 1] Set Player Color/Name and Draw Crosshair
  (Variables|/Script/CoopGame.SHealthComponent|SetbIsDead (Variables|Default|GetHealthComp) false)
  (bind _savegame (|AsyncLoadGamefromSlot "PlayerMenuData")
    (:then
      _)
    (:Completed
      _))
  (bind _asplayer_menu_data (Utilities|Casting|CastToPlayerMenuData _savegame)
    (:then
      _)
    (:CastFailed
      _))
  (Networking|SwitchHasAuthority
    (:Authority
      _)
    (:Remote
      _))
  (Variables|Default|SetPlayColor (Variables|/Game/Blueprints/MainMenu/Blueprints/PlayerMenuData.PlayerMenuData_C|GetPlayerColorSaved _asplayer_menu_data))
  (if (Pawn|IsLocallyControlled)
    (bind _returnvalue (UserInterface|CreateWidget "/Game/UI/WBP_Crosshair.WBP_Crosshair_C"))
    (UserInterface|Viewport|AddtoViewport _returnvalue 0)
    (bind _asplayer_pawn (Utilities|Casting|CastToPlayerPawn (Game|GetPlayerCharacter 0)))
    (CallFunction|SetPlayerName _asplayer_pawn (Variables|/Game/Blueprints/MainMenu/Blueprints/PlayerMenuData.PlayerMenuData_C|GetPlayerNameSaved _asplayer_menu_data))))

(event Game|Damage|EventAnyDamage
  (params (Damage :type Float%20%28single-precision%29) (DamageType :type Damage%20Type%20Object%20Reference) (InstigatedBy :type Controller%20Object%20Reference) (DamageCauser :type Actor%20Object%20Reference))
  ;[1 1 1] Update Health Bar On Damage
  (Utilities|FlowControl|Delay 0.1)
  (bind _asplayer_pawn (Utilities|Casting|CastToPlayerPawn (Game|Player|GetPlayerPawn 0)))
  (CallFunction|SetPlayerHP (/ (Variables|/Script/CoopGame.SHealthComponent|GetHealth (Variables|/Script/CoopGame.SCharacter|GetHealthComp _asplayer_pawn)) 1e+02)))

(event EventTick
  (params (DeltaSeconds :type Float%20%28single-precision%29))
  ;[1 1 1] Update Point HUD
  (bind _asplayer_pawn (Utilities|Casting|CastToPlayerPawn (Game|Player|GetPlayerPawn 0)))
  (Rendering|Components|TextRender|SetText (Variables|Default|Getpoints) (Utilities|Text|ToText(Float) (Variables|/Script/Engine.PlayerState|GetScore (Variables|/Script/Engine.Pawn|GetPlayerState _asplayer_pawn)) "HalfToEven")))

(event EventOnDeath
  ;[1 1 1] On Death
  (bind _assplayer_state (Utilities|Casting|CastToSPlayerState (Variables|Default|GetPlayerState self)))
  (Variables|/Script/CoopGame.SPlayerState|SetPlayerNameState _assplayer_state (Variables|Default|GetPlayerName)))

(event Custom|SetPlayerName
  (params (PlayerNameInput :type String))
  (Variables|Default|SetPlayerName PlayerNameInput))

(event Custom|SetPlayerHP
  (params (HealthInput :type Float%20%28single-precision%29))
  (Variables|Default|SetHealthBar HealthInput))

(event Custom|ServerSetViewTarget
  ;[1 1 1] Get first active player in spectate list. Go to next player on key press, reset if array index out of bounds
  (if (Variables|/Script/CoopGame.SHealthComponent|GetbIsDead (Variables|Default|GetHealthComp))
    (Variables|Default|SetAliveActors (Variables|Default|GetNullArray))
    (CallFunction|GetAlivePlayers)
    (if (Utilities|Array|IsValidIndex (Variables|Default|GetAliveActors) (Variables|Default|GetActivePlayerCamIndex))
      (bind _asplayer_controller (Utilities|Casting|CastToPlayerController (Game|GetPlayerController 0))
        (:then
          (Game|Player|SetViewTargetwithBlend _asplayer_controller (Utilities|Array|Get(acopy) (Variables|Default|GetAliveActors) (Variables|Default|GetActivePlayerCamIndex)) 0.0 "VTBlend_Linear" 0.0 false)
          (bind _result (Math|Integer|IncrementInt (Variables|Default|GetActivePlayerCamIndex))
            (:%20%20
              (Variables|Default|SetActivePlayerCamIndex _result))))
        (:CastFailed
          (Development|PrintString "Cast Failed")))
      (else
        (Variables|Default|SetActivePlayerCamIndex 0)
        (Development|PrintString "bad index")))
    (else
      (Development|PrintString "not dead"))))

(event Custom|Get%20Alive%20Players
  ;[1 1 1] Get List of Living Players For Spectate
  (bind _outactors (Actor|GetAllActorsOfClass "PlayerPawn_C"))
  (for _array_element _outactors
    (if (not (Variables|/Script/CoopGame.SHealthComponent|GetbIsDead (Variables|/Script/CoopGame.SCharacter|GetHealthComp _array_element)))
      (Utilities|Array|Add (Variables|Default|GetAliveActors) _array_element)
      (for _array_element_2 (Variables|Default|GetAliveActors)
        _))))

(event Custom|SpectatePlayers
  ;[1 1 1] Get first active player in spectate list. Go to next player on key press, reset if array index out of bounds
  (Networking|SwitchHasAuthority
    (:Authority
      (if (Variables|/Script/CoopGame.SHealthComponent|GetbIsDead (Variables|Default|GetHealthComp))
        (Variables|Default|SetAliveActors (Variables|Default|GetNullArray))
        (CallFunction|GetAlivePlayers)
        (if (Utilities|Array|IsValidIndex (Variables|Default|GetAliveActors) (Variables|Default|GetActivePlayerCamIndex))
          (bind _asplayer_controller (Utilities|Casting|CastToPlayerController (Game|GetPlayerController 0))
            (:then
              (Game|Player|SetViewTargetwithBlend _asplayer_controller (Utilities|Array|Get(acopy) (Variables|Default|GetAliveActors) (Variables|Default|GetActivePlayerCamIndex)) 0.0 "VTBlend_Linear" 0.0 false)
              (bind _result (Math|Integer|IncrementInt (Variables|Default|GetActivePlayerCamIndex))
                (:%20%20
                  (Variables|Default|SetActivePlayerCamIndex _result))))
            (:CastFailed
              (Development|PrintString "Cast Failed")))
          (else
            (Variables|Default|SetActivePlayerCamIndex 0)
            (Development|PrintString "bad index")))
        (else
          (Development|PrintString "not dead"))))
    (:Remote
      (CallFunction|ServerSetViewTarget))))

(event Input|KeyboardEvents|F
  (params (Key :type Key%20Structure :default "None"))
  ;[1 1 1] Get first active player in spectate list. Go to next player on key press, reset if array index out of bounds
  (:Pressed
    (Networking|SwitchHasAuthority
      (:Authority
        (if (Variables|/Script/CoopGame.SHealthComponent|GetbIsDead (Variables|Default|GetHealthComp))
          (Variables|Default|SetAliveActors (Variables|Default|GetNullArray))
          (CallFunction|GetAlivePlayers)
          (if (Utilities|Array|IsValidIndex (Variables|Default|GetAliveActors) (Variables|Default|GetActivePlayerCamIndex))
            (bind _asplayer_controller (Utilities|Casting|CastToPlayerController (Game|GetPlayerController 0))
              (:then
                (Game|Player|SetViewTargetwithBlend _asplayer_controller (Utilities|Array|Get(acopy) (Variables|Default|GetAliveActors) (Variables|Default|GetActivePlayerCamIndex)) 0.0 "VTBlend_Linear" 0.0 false)
                (bind _result (Math|Integer|IncrementInt (Variables|Default|GetActivePlayerCamIndex))
                  (:%20%20
                    (Variables|Default|SetActivePlayerCamIndex _result))))
              (:CastFailed
                (Development|PrintString "Cast Failed")))
            (else
              (Variables|Default|SetActivePlayerCamIndex 0)
              (Development|PrintString "bad index")))
          (else
            (Development|PrintString "not dead"))))
      (:Remote
        (CallFunction|ServerSetViewTarget)))))

(fn ConstructionScript
  (Rendering|SetOnlyOwnerSee (Variables|Default|Getpoints) true :!class /Script/Engine.PrimitiveComponent))

(fn OnRepPlayColor
  (bind _returnvalue (Rendering|Material|CreateDynamicMaterialInstance (Variables|Character|GetMesh) 0 0 "None" :!class /Script/Engine.PrimitiveComponent))
  (Rendering|Material|SetVectorParameterValue _returnvalue "BodyColor" (Variables|Default|GetPlayColor) :!class /Script/Engine.MaterialInstanceDynamic))

(fn OnRepPlayerName
  ;[1 1 1] Set Player Name Above Player
  (CallFunction|PopulateNameTag (Variables|Default|GetNameTag)))

(fn OnRepHealthBar
  ;[1 1 1] Set Health Value For Health Bar
  (CallFunction|PopulateNameTag (Variables|Default|GetNameTag)))

(fn PopulateNameTag
  (params (Widget :type Widget%20Component%20Object%20Reference))
  (if (not (Networking|IsDedicatedServer))
    (bind _returnvalue (UserInterface|CreateWidget "/Game/Blueprints/Player/PlayerName.PlayerName_C"))
    (UserInterface|SetWidget Widget _returnvalue)
    (Default|UpdatePlayerName _returnvalue (Variables|Default|GetPlayerName))
    (Default|UpdateHealthBar _returnvalue (Variables|Default|GetHealthBar))))